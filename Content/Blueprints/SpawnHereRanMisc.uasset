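; SpawnHereRanMisc is a placeable spawn point that may spawn a random miscellaneous actor at its own transform when play begins.
; On BeginPlay it spawns a SpawnableCollectionMisc helper actor, whose PickRandom supplies the class to spawn.
; SpawnChance acts as the probability by being added to a random roll that must reach one.
; The helper is spawned before the roll and is not destroyed here.
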(event `self.ReceiveBeginPlay`
  (bind _returnvalue (`|SpawnActorFromClass` "/Game/Blueprints/SpawnableCollectionMisc.SpawnableCollectionMisc_C" (`self.GetTransform`) "Undefined" "OverrideRootScale" null null))
  (bind _output_get (set `self.SpawnCollection` _returnvalue))
  (bind _asspawnable_collection_misc (cast `/Game/Blueprints/SpawnableCollectionMisc` _output_get))
  (if (>= (+ (`KismetMathLibrary.RandomFloatInRange` 0.0 1.0) (`self.SpawnChance`)) 1.0)
    (bind _ret (`/Game/Blueprints/SpawnableCollectionMisc.pickRandom` _asspawnable_collection_misc))
    (`|SpawnActorFromClass` _ret (`self.GetTransform`) "Undefined" "OverrideRootScale" null null)))

(fn `UserConstructionScript`)