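; SpawnableCollectionMisc is a Blueprint that holds a collection of miscellaneous spawnable item references, filled in its construction script with the juice carton.
; Check reports whether a given class is in the collection.
; PickRandom walks the collection repeatedly, giving each element a one-in-thirty chance until one is returned, which favours earlier entries and never finishes on an empty collection.
; Its event graph is unused.
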(fn `check`
  (params (classRef :type "Actor Class Reference"))
  (returns (isTrue :type Boolean))
  (locals (NewLocalVar_0 :type Boolean))
  (for _array_element (`self.collection`)
    (if (== _array_element classRef)
      (return true)))
  (return false))

(fn `pickRandom`
  (returns (ret :type "Actor Class Reference"))
  (for _array_element (`self.collection`) :!label _label
    (if (== (`KismetMathLibrary.RandomIntegerInRange` 0 29) 7)
      (return _array_element)))
  (goto _label))

(fn `UserConstructionScript`
  (`KismetArrayLibrary.Array_Add` (`self.collection`) "/Game/Blueprints/Misc/Juice_Carton.Juice_Carton_C"))